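; Fireball actor that explodes once it stops moving vertically, then respawns itself at its starting point.
; Tick adds up time while the Sphere's vertical velocity is near zero, without resetting it during faster motion.
; Past a short threshold, it attaches a child actor and fires a RadialForce impulse.
; After brief delays it hides the boulder mesh, destroys itself and spawns a new Fireball at the location saved on BeginPlay.
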(event EventBeginPlay
  (Variables|Default|SetStarting%20Location (Transformation|GetWorldLocation (Variables|Default|GetSphere self))))

(event Collision|EventActorBeginOverlap
  (params (OtherActor :type Actor%20Object%20Reference)))

(event EventTick
  (params (DeltaSeconds :type Float%20%28single-precision%29))
  (bind _sphere (Variables|Default|GetSphere))
  (bind _radialforce (Variables|Default|GetRadialForce))
  (bind _returnvalue (Transformation|GetComponentVelocity _sphere))
  (if (and (> (.z _returnvalue) -3.0) (< (.z _returnvalue) 3.0))
    (bind _output_get (Variables|Default|SetSlowSeconds (+ DeltaSeconds (Variables|Default|GetSlowSeconds))))
    (if (> _output_get 0.5)
      (Variables|Default|SetSlowSeconds 0.0)
      (AddComponent|AddChildActorComponent false (Math|Transform|MakeTransform "0, 0, 0" "0, 0, 0" "0.500000,0.500000,0.500000"))
      (Variables|/Script/Engine.RadialForceComponent|SetRadius _radialforce 8e+02)
      (Class|RadialForceComponent|FireImpulse _radialforce)
      (Utilities|FlowControl|Delay 0.2)
      (Rendering|SetVisibility (Variables|Default|GetS_Forest_Boulder_wgosajs_lod3_Var1) false false)
      (Utilities|FlowControl|Delay 0.3)
      (Actor|DestroyActor)
      (Game|SpawnActorfromClass "Fireball_C" (Math|Conversions|ToTransform(Vector) (Variables|Default|GetStarting%20Location)) "Undefined" "MultiplyWithRoot" 0 0))))

(fn ConstructionScript)