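; Small slime actor that the player character consumes on touch to gain XP.
; On BeginPlay it caches the player and the mesh's base scale.
; The first player overlap with SlimeyBox awards XP through the player's stats component, zeroes the slime's physics velocity and destroys it after a three-second delay.
; Meanwhile, Tick shrinks it by scaling the base size inversely to accumulated time.
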(event OnComponentBeginOverlap(SlimeyBox)
  (params (OverlappedComponent :type Primitive%20Component%20Object%20Reference) (OtherActor :type Actor%20Object%20Reference) (OtherComp :type Primitive%20Component%20Object%20Reference) (OtherBodyIndex :type Integer) (bFromSweep :type Boolean) (SweepResult :type Hit%20Result%20Structure%20%28by%20ref%29))
  (bind _self self)
  (bind _player (Variables|Default|GetPlayer))
  (bind _bpc_playerstats (Variables|/Game/Blueprints/BP_ThirdPersonCharacter.BP_ThirdPersonCharacter_C|GetBPC_PlayerStats _player))
  ;[1 1 1] Consumed By Main Slime
  (if (and (== (Variables|Default|GetPlayer) OtherActor) (Variables|Default|GetUncontacted))
    (Variables|Default|SetUncontacted false)
    (Default|GainXP _bpc_playerstats (Variables|/Game/Blueprints/BPC_PlayerStats.BPC_PlayerStats_C|GetXP%20per%20slime _bpc_playerstats))
    (Class|PrimitiveComponent|SetAllPhysicsLinearVelocity (Variables|Default|GetOtherSlimes _self) "0, 0, 0" false)
    (Utilities|FlowControl|Delay 3.0)
    (Actor|DestroyActor _self)))

(event EventBeginPlay
  ;[1 1 1] Init Values
  (bind _asbp_third_person_character (Utilities|Casting|CastToBP_ThirdPersonCharacter (Game|GetPlayerCharacter 0)))
  (Variables|Default|SetPlayer _asbp_third_person_character)
  (Variables|Default|SetBaseScale (Variables|/Script/Engine.SceneComponent|GetRelativeScale3D (Variables|Default|GetOtherSlimes))))

(event EventTick
  (params (DeltaSeconds :type Float%20%28single-precision%29))
  ;[1 1 1] Shrink After Contact
  (if (not (Variables|Default|GetUncontacted))
    (bind _output_get (Variables|Default|SetScaleShrinker (+ (Variables|Default|GetScaleShrinker) DeltaSeconds)))
    (Transformation|SetRelativeScale3D (Variables|Default|GetOtherSlimes) (* (Math|Float|SafeDivide 0.75 _output_get) (Variables|Default|GetBaseScale)))))

(fn ConstructionScript)