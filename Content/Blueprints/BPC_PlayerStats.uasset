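; Player stats component that tracks health, XP and level, with debug prints standing in for UI and win/lose screens.
; A looping timer applies heal-over-time, capped at MaxHealth, while damage to zero health triggers game over.
; XP overflow carries into level-ups, which refill health, grow max health linearly and scale jump, size, attack force and range logarithmically.
; Reaching MaxLevel triggers the win and sets a huge XP threshold.
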(event EventBeginPlay
  ;[1 1 1] Heal Over Time system
  (Utilities|Time|SetTimerbyFunctionName 0 "HealOverTime" (Variables|Skills|GetHOT%20rate) true true)
  (Development|PrintString "HOT initiated"))

(event EventTick
  (params (DeltaSeconds :type Float%20%28single-precision%29))
  ;[1 1 1] Update UI
  (Development|PrintString (Utilities|String|ToString(Float) (Variables|Health|GetCurrent%20Health)) true true "(R=1.000000,G=0.000000,B=0.007345,A=1.000000)" 2.0 "1")
  (Development|PrintString (Utilities|String|ToString(Float) (Variables|XP|GetCurrent%20XP)) true true "(R=1.000000,G=0.897633,B=0.000000,A=1.000000)" 2.0 "2")
  (Development|PrintString (Utilities|String|ToString(Integer) (Variables|XP|GetLevel)) true true "(R=1.000000,G=0.380979,B=0.000000,A=1.000000)" 2.0 "3"))

(fn TakeDmg
  (params (Damage :type Float%20%28double-precision%29))
  (bind _output_get (Variables|Health|SetCurrent%20Health (- (Variables|Health|GetCurrent%20Health) Damage)))
  (Development|PrintString (Utilities|String|ToString(Float) Damage) true true "(R=0.244792,G=0.000000,B=0.000000,A=1.000000)")
  (if (<= _output_get 0.0)
    (GameState|GameOver)))

(fn Heal
  (params (Healing :type Float%20%28double-precision%29))
  (bind _output_get (Variables|Health|SetCurrent%20Health (+ (Variables|Health|GetCurrent%20Health) Healing)))
  (Development|PrintString (Utilities|String|ToString(Float) Healing) true true "(R=0.000000,G=1.000000,B=0.181463,A=1.000000)")
  (if (> _output_get (Variables|Health|GetMax%20Health))
    (Variables|Health|SetCurrent%20Health (Variables|Health|GetMax%20Health))))

(fn GainXP
  (params (XP%20Gain :type Float%20%28double-precision%29))
  (bind _output_get (Variables|XP|SetCurrent%20XP (+ (Variables|XP|GetCurrent%20XP) XP%20Gain)))
  (Development|PrintString (Utilities|String|ToString(Float) XP%20Gain))
  (if (>= _output_get (Variables|XP|GetXP%20per%20level))
    ;[1 1 1] overflow XP
    (Variables|XP|SetCurrent%20XP (- (Variables|XP|GetCurrent%20XP) (Variables|XP|GetXP%20per%20level)))
    (XP|LevelUp)))

(fn LevelUp
  (bind _output_get (Variables|XP|SetLevel (+ (Variables|XP|GetLevel) 1)))
  (if (>= _output_get (Variables|XP|GetMax%20Level))
    (GameState|YouWin)
    (Variables|XP|SetXP%20per%20level 1e+07)
    (else
      (bind _stat (XP|JumpMultCalc (Math|Conversions|ToFloat(Integer) _output_get)))
      (Variables|Skills|SetJump%20multiplier _stat)
      (bind _stat_2 (XP|ScaleMultCalc (Math|Conversions|ToFloat(Integer) _output_get)))
      (Variables|Skills|SetScale%20multiplier _stat_2)
      (bind _stat_3 (XP|ForceMultCalc (Math|Conversions|ToFloat(Integer) _output_get)))
      (Variables|Skills|SetAttack%20force%20multiplier _stat_3)
      (bind _stat_4 (XP|RangeMultCalc (Math|Conversions|ToFloat(Integer) _output_get)))
      (Variables|Skills|SetAttack%20range%20multiplier _stat_4)
      (bind _stat_5 (XP|HealthMultCalc (Math|Conversions|ToFloat(Integer) _output_get)))
      (bind _output_get_2 (Variables|Health|SetMax%20Health _stat_5))
      (Variables|Health|SetCurrent%20Health _output_get_2)
      (Variables|XP|SetLevelDing true)
      (Development|PrintString "Level Up"))))

(fn GameOver
  (Development|PrintString "GAME OVER"))

(fn YouWin
  (Development|PrintString "YOU WIN"))

(fn HealOverTime
  (Health|Heal (Variables|Skills|GetHOT%20heal)))

(fn ScaleMultCalc
  (params (Level :type Float%20%28double-precision%29))
  (return (+ (* (Math|Float|Log Level (Math|Conversions|ToFloat(Integer) (Variables|XP|GetMax%20Level))) (Variables|Skills|GetMaxScale)) 1.0)))

(fn ForceMultCalc
  (params (Level :type Float%20%28double-precision%29))
  (return (+ (* (Math|Float|Log Level (Math|Conversions|ToFloat(Integer) (Variables|XP|GetMax%20Level))) (Variables|Skills|GetMaxForce)) 1.0)))

(fn JumpMultCalc
  (params (Level :type Float%20%28double-precision%29))
  (return (+ (* (Math|Float|Log Level (Math|Conversions|ToFloat(Integer) (Variables|XP|GetMax%20Level))) (Variables|Skills|GetMaxJump)) 1.0)))

(fn HealthMultCalc
  (params (Level :type Float%20%28double-precision%29))
  (return (+ (* Level 1e+01) 1e+02)))

(fn RangeMultCalc
  (params (Level :type Float%20%28double-precision%29))
  (return (+ (* (Math|Float|Log Level (Math|Conversions|ToFloat(Integer) (Variables|XP|GetMax%20Level))) (Variables|Skills|GetMaxRange)) 1.0)))