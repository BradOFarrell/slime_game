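; Treasure chest actor that opens when another actor overlaps it.
; Overlap hides the closed chest mesh and shows the open mesh, coins, skull, rect light, cube and decal.
; An Open flag ensures that only the first overlap spawns three child actor components in a short staggered sequence.
; BeginPlay and every overlap also print a debug "Hello".
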(event EventBeginPlay
  (Development|PrintString "Hello"))

(event Collision|EventActorBeginOverlap
  (params (OtherActor :type Actor%20Object%20Reference))
  (Development|PrintString "Hello")
  (Rendering|SetVisibility (Variables|Default|GetSM-Chest-01) false false)
  (Rendering|SetVisibility (Variables|Default|GetSM-Chest-02) true false)
  (if (not (Variables|Default|GetOpen))
    (Variables|Default|SetOpen true)
    (Utilities|FlowControl|Delay 0.2)
    (AddComponent|AddChildActorComponent false)
    (Utilities|FlowControl|Delay 0.2)
    (AddComponent|AddChildActorComponent false)
    (Utilities|FlowControl|Delay 0.2)
    (AddComponent|AddChildActorComponent false)))

(event EventTick
  (params (DeltaSeconds :type Float%20%28single-precision%29)))

(fn ConstructionScript)